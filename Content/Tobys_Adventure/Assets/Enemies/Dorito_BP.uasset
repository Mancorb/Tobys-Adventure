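; Dorito enemy Blueprint that wanders, chases and attacks Toby, and can be killed by his foot.
; It roams random reachable points until PawnSensing spots Toby, then chases with AI MoveTo, returning to roaming after repeated failures or once not attacking.
; Overlapping the attack collision starts a damage loop with randomized attack type and timing.
; When only Toby's left-foot collision overlaps the death collider, it explodes and is destroyed after a short delay.
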(event OnSeePawn(PawnSensing)
  (params (Pawn :type Pawn%20Object%20Reference))
  ;[1 1 1] Chase player
  (Utilities|Casting|CastToToby_BP Pawn)
  (Variables|Default|SetSeenPlayer true)
  (AI|AIMoveTo self "0, 0, 0" Pawn 5.0 false :!label _label
    (:OnSuccess
      (Utilities|FlowControl|Delay 2.0))
    (:OnFail
      (Utilities|FlowControl|Delay 1.0)
      (bind _result (Math|Integer|IncrementInt (Variables|Default|Getmaxfails))
        (:%20%20
          (Variables|Default|Setmaxfails _result)
          (if (>= (Variables|Default|Getmaxfails) 20)
            _
            (else
              (goto _label)))))))
  (Variables|Default|SetSeenPlayer false)
  (if (Variables|Default|GetAttacking)
    (goto _label)
    (else
      ;[1 1 1] AI movement
      (AI|AIMoveTo self (.RandomLocation (AI|Navigation|GetRandomReachablePointinRadius (Transformation|GetActorLocation) (Math|Random|RandomFloatinRange 7e+02 9e+02) 0 0)) 0 5.0 false :!label _label_2
        (:OnSuccess
          (if (not (Variables|Default|GetSeenPlayer))
            (Utilities|FlowControl|Delay (Math|Random|RandomFloatinRange 3.0 5.0))
            (goto _label_2)))))))

(event OnComponentBeginOverlap(Attackcolission)
  (params (OverlappedComponent :type Primitive%20Component%20Object%20Reference) (OtherActor :type Actor%20Object%20Reference) (OtherComp :type Primitive%20Component%20Object%20Reference) (OtherBodyIndex :type Integer) (bFromSweep :type Boolean) (SweepResult :type Hit%20Result%20Structure%20%28by%20ref%29))
  (bind _returnvalue (Math|Random|RandomBool))
  ;[1 1 1] Start Attack
  (bind _astoby_bp (Utilities|Casting|CastToToby_BP OtherActor))
  (Variables|Default|SetAs%20Toby%20BP _astoby_bp)
  (Variables|Default|SetAttacking true)
  (Variables|Default|Setattack%20type _returnvalue :!label _label)
  (if (Math|Boolean|Equal(Boolean) _returnvalue false)
    (Variables|Default|Setdelay 0.42)
    (else
      (Variables|Default|Setdelay 0.32)))
  (Utilities|FlowControl|Delay (Variables|Default|Getdelay))
  (Default|ReduceHealth (Variables|Default|GetAs%20Toby%20BP) (Variables|Default|GetDamage))
  (if (Variables|Default|GetAttacking)
    (Utilities|FlowControl|Delay 0.2)
    (goto _label)))

(event OnComponentEndOverlap(Attackcolission)
  (params (OverlappedComponent :type Primitive%20Component%20Object%20Reference) (OtherActor :type Actor%20Object%20Reference) (OtherComp :type Primitive%20Component%20Object%20Reference) (OtherBodyIndex :type Integer))
  ;[1 1 1] Stop Attack
  (Utilities|Casting|CastToToby_BP OtherActor)
  (Variables|Default|SetAttacking false))

(event OnComponentBeginOverlap(deathcolide)
  (params (OverlappedComponent :type Primitive%20Component%20Object%20Reference) (OtherActor :type Actor%20Object%20Reference) (OtherComp :type Primitive%20Component%20Object%20Reference) (OtherBodyIndex :type Integer) (bFromSweep :type Boolean) (SweepResult :type Hit%20Result%20Structure%20%28by%20ref%29))
  ;[1 1 1] Death
  (bind _astoby_bp (Utilities|Casting|CastToToby_BP OtherActor))
  (Rendering|SetCastShadow (Variables|/Game/Tobys_Adventure/Assets/Character/Toby_BP.Toby_BP_C|GetLeft_foot_collission _astoby_bp) false)
  (if (Utilities|Array|Identical (Class|PrimitiveComponent|GetOverlappingComponents OverlappedComponent) (Utilities|Array|MakeArray (Variables|/Game/Tobys_Adventure/Assets/Character/Toby_BP.Toby_BP_C|GetLeft_foot_collission _astoby_bp)))
    (Variables|Default|Setdead true)
    (Utilities|FlowControl|Delay 0.5)
    (Effects|SpawnEmitteratLocation "/Game/Tobys_Adventure/Assets/particles/simple_explosion.simple_explosion" (Transformation|GetActorLocation self))
    (Actor|DestroyActor)))

(event EventBeginPlay
  ;[1 1 1] AI movement
  (AI|AIMoveTo self (.RandomLocation (AI|Navigation|GetRandomReachablePointinRadius (Transformation|GetActorLocation) (Math|Random|RandomFloatinRange 7e+02 9e+02) 0 0)) 0 5.0 false :!label _label
    (:OnSuccess
      (if (not (Variables|Default|GetSeenPlayer))
        (Utilities|FlowControl|Delay (Math|Random|RandomFloatinRange 3.0 5.0))
        (goto _label)))))

(fn ConstructionScript)