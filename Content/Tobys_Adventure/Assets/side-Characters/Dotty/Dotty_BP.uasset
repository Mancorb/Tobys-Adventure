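; Dotty is a side-character NPC in Toby's Adventure that faces Toby and plays a talk reaction when approached.
; Pawn sensing snaps its full rotation to look at Toby whenever it sees Toby.
; Any actor overlap sets the Talking flag on its Dotty_AB animation instance and plays an interaction cue, and ending overlap clears the flag.
; BeginPlay also creates a hidden Tutorial_2 widget, which this graph never reveals.
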(event OnSeePawn(PawnSensing)
  (params (Pawn :type Pawn%20Object%20Reference))
  (bind _astoby_bp (Utilities|Casting|CastToToby_BP Pawn))
  (Transformation|SetActorRotation (Math|Rotator|FindLookatRotation (Transformation|GetActorLocation) (Transformation|GetActorLocation _astoby_bp))))

(event EventBeginPlay
  ;[1 1 1] Create tutorial widget
  (bind _returnvalue (UserInterface|CreateWidget "/Game/Tobys_Adventure/Lvl_1/UI/Tutorial_2.Tutorial_2_C"))
  (bind _output_get (Variables|Default|Settutorial_2 _returnvalue))
  (UserInterface|Viewport|AddtoViewport _output_get 0)
  (Widget|SetVisibility (Variables|Default|Gettutorial_2) "Hidden"))

(event Collision|EventActorBeginOverlap
  (params (OtherActor :type Actor%20Object%20Reference))
  ;[1 1 1] Show text with sound
  (bind _asdotty_ab (Utilities|Casting|CastToDotty_AB (Components|SkeletalMesh|GetAnimInstance (Variables|Character|GetMesh))))
  (Variables|/Game/Tobys_Adventure/Assets/side-Characters/Dotty/Dotty_AB.Dotty_AB_C|Settalking _asdotty_ab true)
  (Audio|PlaySound2D "/Game/Tobys_Adventure/Assets/sounds/Toby_interaction_Cue.Toby_interaction_Cue" 1.0 1.0 0.0 0 0))

(event EventTick
  (params (DeltaSeconds :type Float%20%28single-precision%29)))

(event Collision|EventActorEndOverlap
  (params (OtherActor :type Actor%20Object%20Reference))
  ;[1 1 1] Show text with sound
  (bind _asdotty_ab (Utilities|Casting|CastToDotty_AB (Components|SkeletalMesh|GetAnimInstance (Variables|Character|GetMesh))))
  (Variables|/Game/Tobys_Adventure/Assets/side-Characters/Dotty/Dotty_AB.Dotty_AB_C|Settalking _asdotty_ab false))

(fn ConstructionScript)