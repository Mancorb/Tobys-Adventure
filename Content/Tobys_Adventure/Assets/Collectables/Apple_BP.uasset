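; Apple_BP is a collectable apple that Toby picks up by overlapping its sphere.
; On overlap with Toby_BP it adds one to the fruit counter and heals him by AmountToHeal.
; It then plays one of three random bite sounds, spawns a small particle burst at its location and destroys itself.
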(event OnComponentBeginOverlap(Sphere)
  (params (OverlappedComponent :type Primitive%20Component%20Object%20Reference) (OtherActor :type Actor%20Object%20Reference) (OtherComp :type Primitive%20Component%20Object%20Reference) (OtherBodyIndex :type Integer) (bFromSweep :type Boolean) (SweepResult :type Hit%20Result%20Structure%20%28by%20ref%29))
  (Variables|Default|Setsound (Math|Random|RandomIntegerinRange 1 3))
  (bind _astoby_bp (Utilities|Casting|CastToToby_BP OtherActor))
  (Variables|/Game/Tobys_Adventure/Assets/Character/Toby_BP.Toby_BP_C|Setfruits_counter _astoby_bp (+ (Variables|/Game/Tobys_Adventure/Assets/Character/Toby_BP.Toby_BP_C|Getfruits_counter _astoby_bp) 1))
  (Default|IncreaseHealth _astoby_bp (Variables|Default|GetAmount%20to%20Heal))
  (if (== (Variables|Default|Getsound) 1)
    (Audio|PlaySound2D "/Game/Tobys_Adventure/Assets/sounds/bite_1_Cue.bite_1_Cue" 1.0 1.0 0.0 0 0)
    (elif (== (Variables|Default|Getsound) 2)
      (Audio|PlaySound2D "/Game/Tobys_Adventure/Assets/sounds/bite_2_Cue.bite_2_Cue" 1.0 1.0 0.0 0 0)
      (else
        (Audio|PlaySound2D "/Game/Tobys_Adventure/Assets/sounds/bite_3_Cue.bite_3_Cue" 1.0 1.0 0.0 0 0))))
  (Effects|SpawnEmitteratLocation "/Game/InfinityBladeEffects/Effects/FX_Treasure/Resources/P_OrePile_Explosion_CrystalPick.P_OrePile_Explosion_CrystalPick" (Transformation|GetActorLocation self) "0, 0, 0" "0.200000,0.200000,0.200000")
  (Actor|DestroyActor))

(fn ConstructionScript)